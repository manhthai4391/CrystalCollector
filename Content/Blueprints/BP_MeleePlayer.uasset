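; BP_MeleePlayer is the player Blueprint that tracks gemstone collection and handles the win and death screens.
; BeginPlay creates the HealthWidget, adds it to the viewport and hides the mouse cursor.
; CollectGemstone increments a counter, playing a pickup sound until the fifth gem triggers PlayerWins instead.
; PlayerWins and PlayerDeath each show their UI through that same widget, then share the step that restores the cursor.
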(event `self.ReceiveBeginPlay`
  (bind _returnvalue (`|CreateWidget` "/Game/UI/HealthWidget.HealthWidget_C"))
  (bind _output_get (set `self.CurrentWidget` _returnvalue))
  (`UserWidget.AddToViewport` _output_get 0)
  (set `PlayerController.bShowMouseCursor` false (`GameplayStatics.GetPlayerController` 0)))

(event `CollectGemstone`
  (bind _output_get (set `self.CollectedGemstone` (+ (`self.CollectedGemstone`) 1)))
  (if (== _output_get 5)
    (`self.PlayerWins`)
    (else
      (`GameplayStatics.PlaySound2D` "/Game/Audio/item-equip-6904.item-equip-6904" 1.0 1.0 0.0 null null))))

(event `PlayerWins`
  (`/Game/UI/HealthWidget.ShowWinUI` (`self.CurrentWidget`))
  (set `PlayerController.bShowMouseCursor` true (`GameplayStatics.GetPlayerController` 0) :!label _label))

(event `PlayerDeath`
  (`/Game/UI/HealthWidget.ShowPlayerDeathUI` (`self.CurrentWidget`))
  (goto _label))

(fn `UserConstructionScript`)